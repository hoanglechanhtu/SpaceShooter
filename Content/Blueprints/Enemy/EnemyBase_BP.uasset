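; Base enemy actor that sweeps in along negative Y on spawn, then bounces back and forth along Z at a randomized speed and starting direction.
; A timeline drives the entry and enables Tick's swept movement when finished.
; Hitting anything but another enemy flips direction and damages the player if struck.
; It registers in GameMode_BP's live-enemy count, decrementing it and destroying itself when health runs out.
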(event `self.ReceiveBeginPlay`
  (bind (_returnvalue_roll _returnvalue_pitch _returnvalue_yaw) (`KismetMathLibrary.BreakRotator` (`self.K2_GetActorRotation`)))
  (bind _spawnlocation (`self.SpawnLocation`))
  ;[1 1 1] Control random move direction
  (bind _asgame_mode_bp (cast `/Game/Blueprints/GameMode_BP` (`GameplayStatics.GetGameMode`)))
  (bind _output_get (set `self.GameMode_BP` _asgame_mode_bp))
  (set `/Game/Blueprints/GameMode_BP.LiveEnemy` (+ (`/Game/Blueprints/GameMode_BP.LiveEnemy` _output_get) 1) _output_get)
  (set `self.bMoveDirection` (`KismetMathLibrary.RandomBool`))
  (set `self.MovementSpeed` (`KismetMathLibrary.RandomFloatInRange` 500.0 1000.0))
  (set `self.SweepIn` (`KismetMathLibrary.RandomFloatInRange` 1200.0 1700.0))
  ;[1 1 1] Spawn Animation
  (set `self.SpawnLocation` (`self.K2_GetActorLocation`))
  (set `self.Yaw` _returnvalue_yaw)
  (bind (_direction _value) (`Timeline|SpawnAnimation`)
    (:`Update`
      (`self.K2_SetActorLocation` (`KismetMathLibrary.VLerp` _spawnlocation (- _spawnlocation (`KismetMathLibrary.MakeVector` 0.0 (`self.SweepIn`))) _value)))
    (:`Finished`
      (set `self.bMoveEnable` true))))

(event `self.ReceiveTick`
  (params (DeltaSeconds :type "Float (single-precision)"))
  ;[1 1 1] Movement
  (if (`self.bMoveEnable`)
    (`self.K2_SetActorLocation` (+ (`self.K2_GetActorLocation`) (* (`KismetMathLibrary.GreaterGreater_VectorRotator` (`KismetMathLibrary.MakeVector` 0.0 0.0 (* (`self.MovementSpeed`) (`KismetMathLibrary.SelectFloat` 1.0 -1.0 (`self.bMoveDirection`))))) DeltaSeconds)) true)))

(event `self.ReceiveHit`
  (params (MyComp :type "PrimitiveComponent Object Reference") (Other :type "Actor Object Reference") (OtherComp :type "PrimitiveComponent Object Reference") (bSelfMoved :type Boolean) (HitLocation :type "Vector Structure") (HitNormal :type "Vector Structure") (NormalImpulse :type "Vector Structure") (Hit :type "HitResult Structure (by ref)"))
  (cast `/Game/Blueprints/Enemy/EnemyBase_BP` Other
    (:`CastFailed`
      (set `self.bMoveDirection` (not (`self.bMoveDirection`)))
      (bind _asplayer_bp (cast `/Game/Blueprints/Player_BP` Other))
      (`GameplayStatics.ApplyDamage` _asplayer_bp 50.0))))

(event `self.ReceiveAnyDamage`
  (params (Damage :type "Float (single-precision)") (DamageType :type "DamageType Object Reference") (InstigatedBy :type "Controller Object Reference") (DamageCauser :type "Actor Object Reference"))
  (bind _gamemode_bp (`self.GameMode_BP`))
  ;[1 1 1] Any damage
  (bind _output_get (set `self.CurrentHealth` (`KismetMathLibrary.FClamp` (- (`self.CurrentHealth`) Damage) 0.0 (`self.MaxHealth`))))
  (if (<= _output_get 0.0)
    (set `/Game/Blueprints/GameMode_BP.LiveEnemy` (- (`/Game/Blueprints/GameMode_BP.LiveEnemy` _gamemode_bp) 1) _gamemode_bp)
    (`self.K2_DestroyActor`)))

(fn `UserConstructionScript`
  (set `self.CurrentHealth` (`self.MaxHealth`)))