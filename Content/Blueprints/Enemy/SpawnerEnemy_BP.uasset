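; Enemy spawner actor that runs three successive waves of enemies.
; A looping timer polls the game mode and starts the next wave when no live enemies remain and the spawner is ready.
; BeginWave publishes the wave size to the game mode, then SpawnWave spawns random classes from that wave's enemy array.
; Spawns share the minimum location's X and Y, with Z randomized between the game mode's bounds.
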(event `self.ReceiveBeginPlay`
  ;[1 1 1] Set wave
  (bind _asgame_mode_bp (cast `/Game/Blueprints/GameMode_BP` (`GameplayStatics.GetGameMode`)))
  (set `self.GameMode_BP` _asgame_mode_bp)
  (bind _returnvalue (`KismetSystemLibrary.K2_SetTimer` null "WaveCheck" 0.5 true))
  (set `self.WaveTimer` _returnvalue))

(event `WaveCheck`
  (bind _output (`|GetArrayItem` (`self.WaveEnemyCount`) (`self.WaveIndex`)))
  (if (and (== (`/Game/Blueprints/GameMode_BP.LiveEnemy` (`self.GameMode_BP`)) 0) (`self.bWaveReady`))
    (switch `int` (`self.WaveIndex`)
      (:`0`
        (`self.BeginWave` _output)
        (`self.SpawnWave` _output (`self.WaveEnemy1`)))
      (:`1`
        (`self.BeginWave` _output)
        (`self.SpawnWave` _output (`self.WaveEnemy2`)))
      (:`2`
        (`self.BeginWave` _output)
        (`self.SpawnWave` _output (`self.WaveEnemy3`))))
    (set `self.WaveIndex` (+ (`self.WaveIndex`) 1))))

(fn `BeginWave`
  (params (WaveTotal :type Integer))
  (bind _gamemode_bp (`self.GameMode_BP`))
  (set `self.bWaveReady` false)
  (set `self.WaveActive` 0)
  (set `/Game/Blueprints/GameMode_BP.MaxWave` WaveTotal _gamemode_bp)
  (set `/Game/Blueprints/GameMode_BP.ActiveWave` WaveTotal _gamemode_bp))

(fn `SpawnWave`
  (params (WaveTotal :type Integer) (WaveEnemy :type "Array of /Game/Blueprints/Enemy/EnemyBase_BP Class Reference"))
  (bind _gamemode_bp (`self.GameMode_BP`))
  (bind (_enemyspawnlocationmax_x _enemyspawnlocationmax_y _enemyspawnlocationmax_z) (`KismetMathLibrary.BreakVector` (`/Game/Blueprints/GameMode_BP.EnemySpawnLocationMax` _gamemode_bp)))
  (bind (_enemyspawnlocationmin_x _enemyspawnlocationmin_y _enemyspawnlocationmin_z) (`KismetMathLibrary.BreakVector` (`/Game/Blueprints/GameMode_BP.EnemySpawnLocationMin` _gamemode_bp)))
  (for _ (range (+ (+ WaveTotal 1) 1))
    (if (> WaveTotal (`self.WaveActive`))
      (if (not (`self.bWaveReady`))
        (`|SpawnActorFromClass` (`|GetArrayItem` WaveEnemy (`KismetMathLibrary.RandomInteger` (`KismetArrayLibrary.Array_Length` WaveEnemy))) (`KismetMathLibrary.MakeTransform` (`KismetMathLibrary.MakeVector` _enemyspawnlocationmin_x _enemyspawnlocationmin_y (`KismetMathLibrary.RandomFloatInRange` _enemyspawnlocationmin_z _enemyspawnlocationmax_z))) "Undefined" "OverrideRootScale" null null)
        (set `self.WaveActive` (+ (`self.WaveActive`) 1)))
      (else
        (set `self.bWaveReady` true)))))

(fn `UserConstructionScript`)