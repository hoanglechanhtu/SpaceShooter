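; Enemy2_BP is an enemy variant that repeatedly fires two projectiles and inherits the rest of its behavior from its parent.
; Tick runs the parent logic, then uses a Delay of FireRate as a repeating fire timer.
; Each cycle spawns stretched ProjectileEnemy_BP shots at the Top and Bottom components, both moving along negative Y.
; The top shot is faster and deals more damage than the bottom one.
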(event `self.ReceiveBeginPlay`
  (`parent.ReceiveBeginPlay`))

(event `self.ReceiveTick`
  (params (DeltaSeconds :type "Float (single-precision)"))
  (`parent.ReceiveTick` DeltaSeconds)
  (`KismetSystemLibrary.Delay` (`self.FireRate`))
  (`|SpawnActorFromClass` "/Game/Blueprints/Projectile/ProjectileEnemy_BP.ProjectileEnemy_BP_C" (`SceneComponent.K2_GetComponentToWorld` (`self.Top`)) "AlwaysSpawn" "OverrideRootScale" null 20.0 (2.5 1.0 1.0) (0.0 -2200.0 0.0) null)
  (`|SpawnActorFromClass` "/Game/Blueprints/Projectile/ProjectileEnemy_BP.ProjectileEnemy_BP_C" (`SceneComponent.K2_GetComponentToWorld` (`self.Bottom`)) "AlwaysSpawn" "OverrideRootScale" null 10.0 (2.5 1.0 1.0) (0.0 -2000.0 0.0) null))

(fn `UserConstructionScript`
  (`parent.UserConstructionScript`))