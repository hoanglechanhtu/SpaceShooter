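; Base player projectile Blueprint that moves at a configurable speed and scale, applied in the construction script.
; On mesh overlap it casts the other actor to its own class as a placeholder for an enemy check.
; If the cast fails, it calls ApplyDamage on the null cast result, so nothing is hurt, then destroys itself.
; Enemy reference, damage class and damage value remain TODOs.
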(event `self.ProjectileMesh.OnComponentBeginOverlap`
  (params (OverlappedComponent :type "PrimitiveComponent Object Reference") (OtherActor :type "Actor Object Reference") (OtherComp :type "PrimitiveComponent Object Reference") (OtherBodyIndex :type Integer) (bFromSweep :type Boolean) (SweepResult :type "HitResult Structure (by ref)"))
  ;[1 1 1] Collision event
  ;;[1 0.09258 0.07268] TODO Replace me with enemy ref
  (bind _asprojectile_player_base_bp (cast `/Game/Blueprints/Projectile/ProjectilePlayerBase_BP` OtherActor)
    (:`CastFailed`
      ;;[1 1 1] TODO create damage class
      (`GameplayStatics.ApplyDamage` _asprojectile_player_base_bp (`self.Damage`))
      (`self.K2_DestroyActor`))))

(fn `UserConstructionScript`
  (bind _projectilemovement (`self.ProjectileMovement`))
  (bind _speed (`self.Speed`))
  (set `ProjectileMovementComponent.InitialSpeed` _speed _projectilemovement)
  (set `ProjectileMovementComponent.MaxSpeed` _speed _projectilemovement)
  (`self.SetActorScale3D` (`self.Scale`)))