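; Enemy projectile actor that flies on its own and damages the player on contact.
; Tick moves it in local space by Speed scaled by delta time, without sweeping.
; A mesh overlap applies Damage only if the other actor is Player_BP, then destroys the projectile whatever it hit.
; The construction script sets the mesh's world scale from the Scale variable.
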(event `self.ReceiveTick`
  (params (DeltaSeconds :type "Float (single-precision)"))
  ;[1 1 1] Movement
  (`self.K2_AddActorLocalOffset` (* (`self.Speed`) DeltaSeconds)))

(event `self.StaticMesh.OnComponentBeginOverlap`
  (params (OverlappedComponent :type "PrimitiveComponent Object Reference") (OtherActor :type "Actor Object Reference") (OtherComp :type "PrimitiveComponent Object Reference") (OtherBodyIndex :type Integer) (bFromSweep :type Boolean) (SweepResult :type "HitResult Structure (by ref)"))
  (bind _asplayer_bp (cast `/Game/Blueprints/Player_BP` OtherActor)
    (:`then`
      (`GameplayStatics.ApplyDamage` _asplayer_bp (`self.Damage`)))
    (:`CastFailed`
      _))
  (`self.K2_DestroyActor`))

(fn `UserConstructionScript`
  (`SceneComponent.SetWorldScale3D` (`self.StaticMesh`) (`self.Scale`)))