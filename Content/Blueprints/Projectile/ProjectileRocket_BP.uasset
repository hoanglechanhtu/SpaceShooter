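; Homing rocket projectile that steers toward the first enemy it detects.
; A HomingBox overlap stores an EnemyBase_BP as the target, replacing it only once the current one is no longer valid.
; Each tick blends the ProjectileMovement velocity halfway toward the target direction scaled by IncreaseSpeed, so the turn rate depends on frame rate.
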(event `self.ReceiveTick`
  (params (DeltaSeconds :type "Float (single-precision)"))
  (`/Engine/EditorBlueprintResources/StandardMacros.IsValid` (`self.Enemy`)
    (:`Is Valid`
      (set `MovementComponent.Velocity` (`KismetMathLibrary.VLerp` (`MovementComponent.Velocity` (`self.ProjectileMovement`)) (* (`KismetMathLibrary.Normal` (- (`self.K2_GetActorLocation` (`self.Enemy`)) (`self.K2_GetActorLocation`))) (`self.IncreaseSpeed`)) 0.5) (`self.ProjectileMovement`)))))

(event `self.HomingBox.OnComponentBeginOverlap`
  (params (OverlappedComponent :type "PrimitiveComponent Object Reference") (OtherActor :type "Actor Object Reference") (OtherComp :type "PrimitiveComponent Object Reference") (OtherBodyIndex :type Integer) (bFromSweep :type Boolean) (SweepResult :type "HitResult Structure (by ref)"))
  ;[1 1 1] Find enemy
  (bind _asenemy_base_bp (cast `/Game/Blueprints/Enemy/EnemyBase_BP` OtherActor))
  (`/Engine/EditorBlueprintResources/StandardMacros.IsValid` (`self.Enemy`)
    (:`Is Not Valid`
      (set `self.Enemy` _asenemy_base_bp))))

(fn `UserConstructionScript`
  (`parent.UserConstructionScript`))