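; Base pickup Blueprint that drifts along world Y at DefaultSpeed until a player comes within its Box, then homes toward them.
; The first Player_BP to overlap the Box is cached as the target while it remains valid.
; Tick sets ProjectileMovement velocity by lerping toward the player direction scaled by IncreaseSpeed, with an Alpha above one that extrapolates rather than smooths.
; The graph contains no collection or reward logic.
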(event `self.ReceiveTick`
  (params (DeltaSeconds :type "Float (single-precision)"))
  (bind _projectilemovement (`self.ProjectileMovement`))
  ;[1 1 1] Movement Control
  (`/Engine/EditorBlueprintResources/StandardMacros.IsValid` (`self.Player_BP`)
    (:`Is Valid`
      (set `MovementComponent.Velocity` (`KismetMathLibrary.VLerp` (`MovementComponent.Velocity` _projectilemovement) (* (`KismetMathLibrary.Normal` (- (`self.K2_GetActorLocation` (`self.Player_BP`)) (`self.K2_GetActorLocation`))) (`self.IncreaseSpeed`)) 10.0) _projectilemovement))
    (:`Is Not Valid`
      (set `MovementComponent.Velocity` (`KismetMathLibrary.MakeVector` 0.0 (`self.DefaultSpeed`)) _projectilemovement))))

(event `self.Box.OnComponentBeginOverlap`
  (params (OverlappedComponent :type "PrimitiveComponent Object Reference") (OtherActor :type "Actor Object Reference") (OtherComp :type "PrimitiveComponent Object Reference") (OtherBodyIndex :type Integer) (bFromSweep :type Boolean) (SweepResult :type "HitResult Structure (by ref)"))
  ;[1 1 1] Overlap control
  (bind _asplayer_bp (cast `/Game/Blueprints/Player_BP` OtherActor))
  (`/Engine/EditorBlueprintResources/StandardMacros.IsValid` (`self.Player_BP`)
    (:`Is Not Valid`
      (set `self.Player_BP` _asplayer_bp))))

(fn `UserConstructionScript`)