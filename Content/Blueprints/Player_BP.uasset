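; Player pawn for a shooter with movement in the Y-Z plane, starting with a timeline fly-in that then enables control.
; Tick eases input into speed, applies swept moves and pitches the mesh with vertical speed.
; Input-held gates and cooldowns drive primary, power-up and rocket fire; the latter two spawn Player_BP itself rather than projectiles.
; Damage drains clamped health; at zero it flags PlayerDead on GameMode_BP and destroys the actor.
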(event `self.ReceiveBeginPlay`
  (bind _spawnlocation (`self.SpawnLocation`))
  ;[1 0.915 0.06639] Spawn namition
  (set `self.CurrentHealth` (`self.MaxHealth`))
  (set `self.Pitch` (.pitch (`SceneComponent.RelativeRotation` (`self.PlayerMesh`))))
  (set `self.SpawnLocation` (`self.K2_GetActorLocation`))
  (set `self.SpawnRotation` (`SceneComponent.K2_GetComponentRotation` (`self.PlayerMesh`)))
  (bind (_direction _spawn) (`Timeline|SpawnAnimation`)
    (:`Update`
      (`self.K2_SetActorLocation` (`KismetMathLibrary.VLerp` _spawnlocation (+ _spawnlocation (0.0 1000.0 0.0)) _spawn))
      (`SceneComponent.K2_SetRelativeRotation` (`self.PlayerMesh`) (`KismetMathLibrary.RLerp` (`self.SpawnRotation`) (`KismetMathLibrary.MakeRotator` 0.0 (+ (`self.AnimationPitch`) (`self.Pitch`))) _spawn) false false))
    (:`Finished`
      (set `self.bMovementEnable` true))))

(event `self.ReceiveTick`
  (params (DeltaSeconds :type "Float (single-precision)"))
  ;[0 0.452 1] Movement
  (set `self.DeltaSecond` DeltaSeconds)
  (if (`self.bMovementEnable`)
    (`self.FireRateControl`)
    (`|ExecutionSequence`
      (:`then_0`
        (bind _returndirection (`self.GetDirection` (`self.VertSpeed`) (`self.GetInputAxisValue`)))
        (set `self.VertSpeed` _returndirection))
      (:`then_1`
        (bind _returndirection_2 (`self.GetDirection` (`self.HozSpeed`) (`self.GetInputAxisValue`)))
        (set `self.HozSpeed` _returndirection_2))
      (:`then_2`
        (`self.K2_SetActorLocation` (+ (`self.K2_GetActorLocation`) (`KismetMathLibrary.MakeVector` 0.0 0.0 (`self.VertSpeed`))) true)
        (`self.K2_SetActorLocation` (+ (`self.K2_GetActorLocation`) (`KismetMathLibrary.MakeVector` 0.0 (`self.HozSpeed`))) true)
        (if (> (`self.CurrentHealth`) 0.0)
          (`SceneComponent.K2_SetRelativeRotation` (`self.PlayerMesh`) (`KismetMathLibrary.RInterpTo` (`self.K2_GetActorRotation`) (`KismetMathLibrary.MakeRotator` 0.0 (* (`self.VertSpeed`) 4.0)) (`self.DeltaSecond`) 20.0) false false))))))

(event `FireRateControl`
  (bind _projectilespawn (`self.ProjectileSpawn`))
  ;[1 0 0.1187] Projectile control
  (`|ExecutionSequence`
    (:`then_0`
      (bind _output_get (set `self.PrimaryFireRate` (- (`self.PrimaryFireRate`) (`self.DeltaSecond`))))
      (if (<= _output_get 0.0)
        (`/Engine/EditorBlueprintResources/StandardMacros.Gate` true :!label _label
          (:`Exit`
            (set `self.PrimaryFireRate` (`self.PrimaryFireRateBase`))
            (if (not (`self.bHasPower`))
              (`self.PrimaryFire` _projectilespawn)
              (else
                (`self.PowerUpFire` (`self.NumberOfShots`) _projectilespawn)))))))
    (:`then_1`
      (bind _output_get_2 (set `self.SecondaryFireRate ` (- (`self.SecondaryFireRate `) (`self.DeltaSecond`))))
      (if (<= _output_get_2 0.0)
        (`/Engine/EditorBlueprintResources/StandardMacros.Gate` true :!label _label_2
          (:`Exit`
            (set `self.SecondaryFireRate ` (`self.SecondaryFireRateBase`))
            (if (`self.bHasRocket`)
              (`self.SecondaryFire` (`self.NumberOfRocketShots`) _projectilespawn))))))))

(event `InputAction|PrimaryFire`
  (params (Key :type "Key Structure"))
  ;[1 0 0.1187] Projectile control
  (:`Pressed`
    (goto _label :!via `Open`))
  (:`Released`
    (goto _label :!via `Close`)))

(event `InputAction|RocketFire`
  (params (Key :type "Key Structure"))
  ;[1 0 0.1187] Projectile control
  (:`Pressed`
    (goto _label_2 :!via `Open`))
  (:`Released`
    (goto _label_2 :!via `Close`)))

(event `self.ReceiveAnyDamage`
  (params (Damage :type "Float (single-precision)") (DamageType :type "DamageType Object Reference") (InstigatedBy :type "Controller Object Reference") (DamageCauser :type "Actor Object Reference"))
  ;[1 1 1] Control player deadth
  (bind _output_get (set `self.CurrentHealth` (`KismetMathLibrary.FClamp` (- (`self.CurrentHealth`) Damage) 0.0 (`self.MaxHealth`))))
  (if (<= _output_get 0.0)
    (bind _asgame_mode_bp (cast `/Game/Blueprints/GameMode_BP` (`GameplayStatics.GetGameMode`)))
    (set `/Game/Blueprints/GameMode_BP.bPlayerDead` true _asgame_mode_bp)
    (`self.K2_DestroyActor`)))

(fn `GetDirection`
  (params (Speed :type "Float (double-precision)") (Direction :type "Float (double-precision)"))
  (returns (ReturnDirection :type "Float (double-precision)"))
  (bind _output_get (set `self.CurrentSpeed` (`KismetMathLibrary.FInterpTo` Speed (* Direction (`self.MovementSpeed`)) (`self.DeltaSecond`) 4.0)))
  (return _output_get))

(fn `PowerUpFire`
  (params (NumberOfShots :type Integer) (SpawnLocation :type "SceneComponent Object Reference (by ref)"))
  (locals (Offset :type Integer))
  (bind _returnvalue (`SceneComponent.K2_GetComponentToWorld` SpawnLocation))
  (bind _returnvalue_2 (* (`KismetMathLibrary.Conv_IntToDouble` (`local.Offset`)) 5.0))
  (set `local.Offset` (/ NumberOfShots -2))
  (for _ (range (+ NumberOfShots 1))
    (`|SpawnActorFromClass` "Player_BP_C" (`KismetMathLibrary.MakeTransform` (`KismetMathLibrary.MakeVector` (.x (.location _returnvalue)) (.y (.location _returnvalue)) (+ (.z (.location _returnvalue)) _returnvalue_2)) (`KismetMathLibrary.MakeRotator` _returnvalue_2)) "AlwaysSpawn" "OverrideRootScale" null null)
    (set `local.Offset` (+ (`local.Offset`) 1))))

(fn `PrimaryFire`
  (params (SpawnLocation :type "SceneComponent Object Reference"))
  (`|SpawnActorFromClass` "/Game/Blueprints/Projectile/ProjectilePrimary_BP.ProjectilePrimary_BP_C" (`KismetMathLibrary.MakeTransform` (`KismetMathLibrary.MakeVector` (.x (.location (`SceneComponent.K2_GetComponentToWorld` SpawnLocation))) (.y (.location (`SceneComponent.K2_GetComponentToWorld` SpawnLocation))) (+ (.z (.location (`SceneComponent.K2_GetComponentToWorld` SpawnLocation))) (`KismetMathLibrary.RandomFloatInRange` -70.0 70.0))) (.rotation (`SceneComponent.K2_GetComponentToWorld` SpawnLocation))) "AlwaysSpawn" "OverrideRootScale" null null))

(fn `SecondaryFire`
  (params (NumberOfShots :type Integer) (SpawnLocation :type "SceneComponent Object Reference (by ref)"))
  (locals (Offset :type Integer))
  (bind _returnvalue (`SceneComponent.K2_GetComponentToWorld` SpawnLocation))
  (bind _returnvalue_2 (* (`KismetMathLibrary.Conv_IntToDouble` (`local.Offset`)) 5.0))
  (set `local.Offset` (/ (+ NumberOfShots 1) -1))
  (for _ (range (+ NumberOfShots 1))
    (`|SpawnActorFromClass` "Player_BP_C" (`KismetMathLibrary.MakeTransform` (`KismetMathLibrary.MakeVector` (.x (.location _returnvalue)) (.y (.location _returnvalue)) (+ (.z (.location _returnvalue)) _returnvalue_2)) (`KismetMathLibrary.MakeRotator` _returnvalue_2)) "AlwaysSpawn" "OverrideRootScale" null null)
    (set `local.Offset` (+ (`local.Offset`) 4))))

(fn `UserConstructionScript`)